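; A button Blueprint that spawns a small random batch of UFO actors when pressed.
; It extends the parent's ButtonPressed event, calling the parent first and then looping to spawn the UFOs.
; Each spawn location is a random point in bounds built from the Box1 component's world location and its scaled extent rotated by its world rotation.
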(event EventBeginPlay)

(event Collision|EventActorBeginOverlap
  (params (OtherActor :type Actor%20Object%20Reference))
  (|CallParentFunction OtherActor) ; This node is disabled and will not be called.\nDrag off pins to build functionality.
)

(event EventTick
  (params (DeltaSeconds :type Float%20%28single-precision%29)))

(event EventButtonPressed
  (bind _box1 (Variables|Default|GetBox1))
  (|CallParentFunction)
  (for _index (range 0 (Math|Random|RandomIntegerinRange 2 5))
    (Game|SpawnActorfromClass "/Game/UFO.UFO_C" (Math|Transform|MakeTransform (Math|Random|RandomPointinBoundingBox (Transformation|GetWorldLocation _box1) (Math|Vector|RotateVector (Components|Box|GetScaledBoxExtent _box1) (Transformation|GetWorldRotation _box1))) "0, 0, 0" "1,1,1") "Undefined" 0 0)))

(fn ConstructionScript
  (|CallParentFunction))